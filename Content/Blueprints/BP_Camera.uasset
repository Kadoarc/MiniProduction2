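; Shared camera for up to four local players that follows the group and zooms to their spread.
; After a short delay it takes the players from BP_Local_GameMode, numbers them and makes itself the player controllers' view target.
; A fast looping timer, rather than Tick, sets spring arm length from the largest pairwise distance, clamped.
; It also moves the camera at constant speed toward the players' offset average position, with fixed height.
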(event `self.ReceiveBeginPlay`
  (`KismetSystemLibrary.Delay` 0.2)
  (`self.ClassSetup`)
  (`KismetSystemLibrary.K2_SetTimer` null "UpdateCamera" 0.001 true))

(event `UpdateCamera`
  (`self.SetArmLength`)
  (`self.SetCameraPos`))

(fn `CalculateDistance`
  (params (PlayerRef1 :type "/Game/Blueprints/BP_Player_Character Object Reference") (PlayerRef2 :type "/Game/Blueprints/BP_Player_Character Object Reference"))
  (returns (Distance1 :type "Float (double-precision)"))
  (locals (Distance :type "Float (double-precision)" :default 0.0))
  (if (and (`KismetSystemLibrary.IsValid` PlayerRef1) (`KismetSystemLibrary.IsValid` PlayerRef2))
    (set `local.Distance` (`self.GetDistanceTo` PlayerRef1 PlayerRef2))
    (else
      (set `local.Distance` 0.0)))
  (return (`local.Distance`)))

(fn `ClassSetup`
  (bind _asbp_local_game_mode (cast `/Game/Blueprints/BP_Local_GameMode` (`GameplayStatics.GetGameMode`)))
  (set `self.PlayersReference` (`/Game/Blueprints/BP_Local_GameMode.Players` _asbp_local_game_mode))
  ;[1 1 1] Get each players player controller, set their view target to BP_Camera(SELF)
  (bind _outactors (`GameplayStatics.GetAllActorsOfClass` "/Script/Engine.PlayerController"))
  (`PlayerController.SetViewTargetWithBlend` _outactors self 0.0 "VTBlend_Linear" 0.0 false)
  (for (_array_element _array_index) (`self.PlayersReference`)
    (switch `int` _array_index
      (:`0`
        (bind _output_get (set `self.P1` _array_element))
        (set `/Game/Blueprints/BP_Player_Character.PlayerNumber` 0 _output_get))
      (:`1`
        (bind _output_get_2 (set `self.P2` _array_element))
        (set `/Game/Blueprints/BP_Player_Character.PlayerNumber` 1 _output_get_2))
      (:`2`
        (bind _output_get_3 (set `self.P3` _array_element))
        (set `/Game/Blueprints/BP_Player_Character.PlayerNumber` 2 _output_get_3))
      (:`3`
        (bind _output_get_4 (set `self.P4` _array_element))
        (set `/Game/Blueprints/BP_Player_Character.PlayerNumber` 3 _output_get_4)))))

(fn `GetLocation`
  (params (Player :type "/Game/Blueprints/BP_Player_Character Object Reference"))
  (returns (Location1 :type "Vector Structure"))
  (locals (Location :type "Vector Structure" :default (0.0 0.0 0.0)))
  (`/Engine/EditorBlueprintResources/StandardMacros.IsValid` Player
    (:`Is Valid`
      (set `local.Location` (`self.K2_GetActorLocation` Player)))
    (:`Is Not Valid`
      (set `local.Location` (0.0 0.0 0.0))))
  (return (`local.Location`)))

(fn `SetArmLength`
  (bind _p1 (`self.P1`))
  (bind _p2 (`self.P2`))
  (bind _p3 (`self.P3`))
  (bind _p4 (`self.P4`))
  (set `SpringArmComponent.TargetArmLength` (`KismetMathLibrary.FClamp` (`.MaxValue` (`KismetMathLibrary.MaxOfFloatArray` (`|MakeArray` (`self.CalculateDistance` _p1 _p2) (`self.CalculateDistance` _p1 _p3) (`self.CalculateDistance` _p1 _p4) (`self.CalculateDistance` _p2 _p3) (`self.CalculateDistance` _p2 _p4) (`self.CalculateDistance` _p3 _p4)))) (`self.MinArmLength`) (`self.MaxArmLength`)) (`self.SpringArm`)))

(fn `SetCameraPos`
  (bind (_returnvalue_x _returnvalue_y) (`KismetMathLibrary.BreakVector` (`KismetMathLibrary.VInterpTo_Constant` (`self.PreviousPos`) (`self.TargetPos`) (`GameplayStatics.GetWorldDeltaSeconds`) 60.0)))
  (set `self.TargetPos` (- (/ (+ (`self.GetLocation` (`self.P1`)) (`self.GetLocation` (`self.P2`)) (`self.GetLocation` (`self.P3`)) (`self.GetLocation` (`self.P4`))) (`KismetMathLibrary.Conv_IntToDouble` (`KismetArrayLibrary.Array_Length` (`self.PlayersReference`)))) (200.0 0.0 0.0)))
  (`self.K2_SetActorLocation` (`KismetMathLibrary.MakeVector` _returnvalue_x _returnvalue_y -500.0))
  (set `self.PreviousPos` (`self.K2_GetActorLocation`)))

(fn `UserConstructionScript`)