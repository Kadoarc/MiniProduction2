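; Game mode for a local multiplayer Hot Potato minigame where bomb holders are eliminated until one player remains.
; InitialiseGame spawns and possesses a character per GameInstance player at tagged PlayerStarts, assigning husky skins, then resets control rotations.
; BlowUpBomb destroys the holder with effects, calls GiveRandomPlayerBomb and reschedules itself by timer.
; GiveRandomPlayerBomb picks a survivor, or triggers GameOver, blending the camera to the winner.
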(event `GameOver`
  (params (ch :type "/Game/Blueprints/BP_Player_Character_HotPotato Object Reference"))
  (`KismetSystemLibrary.PrintString` "Game Over")
  ;[1 1 1] Get the personal camera actor and update it
  (bind _outactors (`GameplayStatics.GetAllActorsOfClass` "/Game/Blueprints/Cameras/BP_PersonalCamera.BP_PersonalCamera_C"))
  (bind _output (`|GetArrayItem` _outactors))
  (`/Game/Blueprints/Cameras/BP_PersonalCamera.UpdatePersonalCamera` _output null ch false)
  ;[1 1 1] Transition the camera to the winner
  (`PlayerController.SetViewTargetWithBlend` (`GameplayStatics.GetPlayerController` 0) _output 1.0 "VTBlend_EaseIn" 1.0 false))

(event `InitialiseGame`
  (`|ExecutionSequence`
    (:`then_0`
      (`self.GetPlayerStartPoints`))
    (:`then_1`
      (`self.SpawnPlayers`))
    (:`then_2`
      (`self.SetPlayerInitialRotations`))
    (:`then_3`
      (bind _asbp_game_instance (cast `/Game/Blueprints/GameModes/BP_GameInstance` (`GameplayStatics.GetGameInstance`)))
      (set `self.RemainingPlayers` (`/Game/Blueprints/GameModes/BP_GameInstance.TotalPlayers` _asbp_game_instance)))))

(fn `BlowUpBomb`
  (bind _outactors (`GameplayStatics.GetAllActorsOfClass` "/Game/Blueprints/BP_Player_Character_HotPotato.BP_Player_Character_HotPotato_C"))
  (for _array_element _outactors
    (bind _asbp_player_character_hot_potato (cast `/Game/Blueprints/BP_Player_Character_HotPotato` (`GameplayStatics.GetPlayerCharacter` (`/Game/Blueprints/BP_Player_Character_HotPotato.PlayerNumber` _array_element))))
    (if (`/Game/Blueprints/BP_Player_Character_HotPotato.HasBomb?` _asbp_player_character_hot_potato)
      (`GameplayStatics.SpawnEmitterAtLocation` "/Game/ParticleEffects/IcicleExplosion_PAR.IcicleExplosion_PAR" (`self.K2_GetActorLocation` _asbp_player_character_hot_potato))
      (`self.K2_DestroyActor` _asbp_player_character_hot_potato)
      (`GameplayStatics.PlaySound2D` "/Game/Assets/Audio/BombExplode.BombExplode" 1.0 1.0 0.0 null null)
      (bind _result (`/Engine/EditorBlueprintResources/StandardMacros.DecrementInt` (stale _output_get))
        (:`  `
          (bind _output_get (set `self.RemainingPlayers` _result))
          (`self.GiveRandomPlayerBomb`)
          (`KismetSystemLibrary.K2_SetTimer` null "BlowUpBomb" 5.0)
          (`KismetSystemLibrary.PrintString` (`KismetStringLibrary.Concat_StrStr` "Remaining Players: " (`KismetStringLibrary.Conv_IntToString` _output_get)) true true (struct :`G` 0.66 :`B` 1.0 :`A` 1.0) 5.0))))))

(fn `GetPlayerStartPoints`
  (bind _outactors (`GameplayStatics.GetAllActorsOfClass` "/Script/Engine.PlayerStart"))
  (set `self.PlayerStartArray` _outactors))

(fn `GiveRandomPlayerBomb`
  (`/Engine/EditorBlueprintResources/StandardMacros.DoOnce` false :!label _label
    (:`Completed`
      (bind _result (`/Engine/EditorBlueprintResources/StandardMacros.IncrementInt` (`self.DebugLog`))
        (:`  `
          (`KismetSystemLibrary.PrintString` (`KismetStringLibrary.Concat_StrStr` "[DEBUG CALL]: # " (`KismetStringLibrary.Conv_IntToString` _result)) true true (struct :`G` 0.66 :`B` 1.0 :`A` 1.0) 10.0)
          (bind _outactors (`GameplayStatics.GetAllActorsOfClass` "/Game/Blueprints/BP_Player_Character_HotPotato.BP_Player_Character_HotPotato_C"))
          (bind _returnvalue (`KismetArrayLibrary.Array_LastIndex` _outactors))
          (if (== _returnvalue 0)
            (`self.GameOver` (`|GetArrayItem` _outactors _returnvalue))
            (else
              (bind _asbp_player_character_hot_potato (cast `/Game/Blueprints/BP_Player_Character_HotPotato` (`GameplayStatics.GetPlayerCharacter` (`/Game/Blueprints/BP_Player_Character_HotPotato.PlayerNumber` (`|GetArrayItem` _outactors (`KismetMathLibrary.RandomIntegerInRange` 0 _returnvalue)))))
                (:`then`
                  (set `/Game/Blueprints/BP_Player_Character_HotPotato.HasBomb?` true _asbp_player_character_hot_potato)
                  (`SceneComponent.ToggleVisibility` (`/Game/Blueprints/BP_Player_Character_HotPotato.BombIndicator` _asbp_player_character_hot_potato) false)
                  (`KismetSystemLibrary.PrintString` (`KismetStringLibrary.Concat_StrStr` "Player: " (`KismetStringLibrary.Conv_IntToString` (+ (`/Game/Blueprints/BP_Player_Character_HotPotato.PlayerNumber` _asbp_player_character_hot_potato) 1)) " has the bomb.") true true (struct :`G` 0.66 :`B` 1.0 :`A` 1.0) 10.0)
                  (goto _label :!via `Reset`))
                (:`CastFailed`
                  (`KismetSystemLibrary.PrintString` "Cast Failed"))))))))))

(fn `Init Timer`
  (params (`Time To Complete` :type "Float (double-precision)" :default 0.0))
  (set `self.Time Remaining` `Time To Complete`)
  (bind _returnvalue (`KismetSystemLibrary.K2_SetTimer` null "Refresh Timer" (`self.Timer Tick Delta`) true))
  (set `self.Main Timer Handle` _returnvalue))

(fn `Refresh Timer`)

(fn `SetPlayerInitialRotations`
  ;[1 1 1] -Get each player;
  ; -Change controller to respond to normal vector values;
  ; // This is because the player start has been rotated for each
  ; player and the controls will not be aligned otherwise;
  (bind _outactors (`GameplayStatics.GetAllActorsOfClass` "/Game/Blueprints/BP_Player_Character_HotPotato.BP_Player_Character_HotPotato_C"))
  (for (_ _array_index) _outactors
    (`Controller.SetControlRotation` (`GameplayStatics.GetPlayerController` _array_index) (`KismetMathLibrary.Conv_Vector4ToRotator` (`KismetMathLibrary.MakeVector4` 0.0)))))

(fn `SpawnPlayers`
  (bind _index (`self.Index`))
  (bind _asbp_game_instance (cast `/Game/Blueprints/GameModes/BP_GameInstance` (`GameplayStatics.GetGameInstance`)))
  ;[0.4158 1 0.9701] Array is zero based, update for normal 1-4 use.
  (for _index_2 (range (`/Game/Blueprints/GameModes/BP_GameInstance.TotalPlayers` _asbp_game_instance))
    (set `self.Index` _index_2)
    ;[0.4374 1 0.9901] Assign each player from the array with the player start tag
    (for _array_element (`self.PlayerStartArray`)
      (if (== (`PlayerStart.PlayerStartTag` _array_element) (`KismetStringLibrary.Conv_StringToName` (`KismetStringLibrary.Conv_IntToString` (`self.Index`))))
        ;[0.4256 1 0.9602] Spawn the BP_Player and assign the player to posses it
        (bind _returnvalue (`GameplayStatics.CreatePlayer` (`self.Index`)))
        (bind _returnvalue_2 (`|SpawnActorFromClass` "/Game/Blueprints/BP_Player_Character_HotPotato.BP_Player_Character_HotPotato_C" (`self.GetTransform` _array_element) "Undefined" "OverrideRootScale" _returnvalue null))
        (`Controller.Possess` (`GameplayStatics.GetPlayerController` _index) _returnvalue_2)
        ;[1 1 1] Add each unique element to the players array
        (`KismetArrayLibrary.Array_AddUnique` (`self.Players`))
        ;[0.2696 0.9602 1] Change the mesh and animations based on player index
        (switch `int` _index
          (:`0`
            (bind _mesh (`Character.Mesh` _returnvalue_2))
            (`SkinnedMeshComponent.SetSkinnedAssetAndUpdate` _mesh "/Game/NEW_Assets/Characters/FairyHusky/Animations/FairyHuskyIdle_anim.FairyHuskyIdle_anim" true)
            (`SkeletalMeshComponent.K2_SetAnimInstanceClass` _mesh "/Game/NEW_Assets/Characters/FairyHusky/Animations/ABP_Fairy.ABP_Fairy_C")
            (set `/Game/Blueprints/BP_Player_Character_HotPotato.PlayerNumber` 0 _returnvalue_2)
            (`StaticMeshComponent.SetStaticMesh` (`/Game/Blueprints/BP_Player_Character_HotPotato.PlayerIndicator ` _returnvalue_2) "/Game/Assets/Crystals/Crystal_FairyHusky.Crystal_FairyHusky"))
          (:`1`
            (bind _mesh_2 (`Character.Mesh` _returnvalue_2))
            (`SkinnedMeshComponent.SetSkinnedAssetAndUpdate` _mesh_2 "/Game/NEW_Assets/Characters/HuskMitri/Animations/HuskmitriIdle_anim.HuskmitriIdle_anim" true)
            (`SkeletalMeshComponent.K2_SetAnimInstanceClass` _mesh_2 "/Game/NEW_Assets/Characters/HuskMitri/Animations/ABP_HuskMitri.ABP_HuskMitri_C")
            (set `/Game/Blueprints/BP_Player_Character_HotPotato.PlayerNumber` 1 _returnvalue_2)
            (`StaticMeshComponent.SetStaticMesh` (`/Game/Blueprints/BP_Player_Character_HotPotato.PlayerIndicator ` _returnvalue_2) "/Game/Assets/Crystals/Crystal_HuskyMitri.Crystal_HuskyMitri"))
          (:`2`
            (bind _mesh_3 (`Character.Mesh` _returnvalue_2))
            (`SkinnedMeshComponent.SetSkinnedAssetAndUpdate` _mesh_3 "/Game/NEW_Assets/Characters/PunkHusky/PunkHuskyIdle_anim.PunkHuskyIdle_anim" true)
            (`SkeletalMeshComponent.K2_SetAnimInstanceClass` _mesh_3 "/Game/NEW_Assets/Characters/PunkHusky/ABP_Punk.ABP_Punk_C")
            (set `/Game/Blueprints/BP_Player_Character_HotPotato.PlayerNumber` 2 _returnvalue_2)
            (`StaticMeshComponent.SetStaticMesh` (`/Game/Blueprints/BP_Player_Character_HotPotato.PlayerIndicator ` _returnvalue_2) "/Game/Assets/Crystals/Crystal_HuskyPunk.Crystal_HuskyPunk"))
          (:`3`
            (bind _mesh_4 (`Character.Mesh` _returnvalue_2))
            (`SkinnedMeshComponent.SetSkinnedAssetAndUpdate` _mesh_4 "/Game/NEW_Assets/Characters/SwimmerHusky/SwimmerHuskyIdle_anim.SwimmerHuskyIdle_anim" true)
            (`SkeletalMeshComponent.K2_SetAnimInstanceClass` _mesh_4 "/Game/NEW_Assets/Characters/SwimmerHusky/ABP_Swimmer.ABP_Swimmer_C")
            (set `/Game/Blueprints/BP_Player_Character_HotPotato.PlayerNumber` 3 _returnvalue_2)
            (`StaticMeshComponent.SetStaticMesh` (`/Game/Blueprints/BP_Player_Character_HotPotato.PlayerIndicator ` _returnvalue_2) "/Game/Assets/Crystals/Crystal_HuskySwimmer.Crystal_HuskySwimmer")))))))

(fn `UserConstructionScript`)