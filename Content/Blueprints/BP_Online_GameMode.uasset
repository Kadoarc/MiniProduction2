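; Online game mode that gathers PlayerStarts on BeginPlay and logs controller IDs on login.
; ChoosePlayerStart hands out each start once by removing it from the cached array.
; SpawnPlayers, uncalled here, creates local players at index-tagged starts, possessing characters styled as bear, fox, penguin or walrus with colored cone indicators.
; Several overrides are stubs: ReadyToStartMatch returns false, default pawn spawning returns nothing, and SetPlayerInitialRotations only touches player 0.
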(event `self.ReceiveBeginPlay`
  (`self.GetPlayerStartPoints`))

(event `self.K2_PostLogin`
  (params (NewPlayer :type "PlayerController Object Reference"))
  (`KismetSystemLibrary.PrintString` (`KismetStringLibrary.Concat_StrStr` "Player Controller ID #" (`KismetStringLibrary.Conv_IntToString` (`GameplayStatics.GetPlayerControllerID` NewPlayer)) " OnPostLogin") true true (struct :`R` 1.0 :`B` 0.034265 :`A` 1.0) 10.0))

(fn `ChoosePlayerStart`
  (params (Player :type "Controller Object Reference"))
  (returns (ReturnValue :type "Actor Object Reference"))
  (bind _playerstartarray (`self.PlayerStartArray`))
  (if (not (`self.Gathered Player Start Points ?`))
    ;[1 0.2592 0.2393] Get an array of the player start points
    (bind _outactors (`GameplayStatics.GetAllActorsOfClass` "/Script/Engine.PlayerStart"))
    (set `self.PlayerStartArray` _outactors)
    (set `self.Gathered Player Start Points ?` true))
  ;[0.3846 1 0.4252] Get the player start based on the # of players spawned, then remove it from the array before returning the spawn point
  (bind _output_get (set `self.Selected Player Start` (`|GetArrayItem` _playerstartarray (stale _result))))
  (`KismetArrayLibrary.Array_RemoveItem` _playerstartarray _output_get)
  (bind _result (`/Engine/EditorBlueprintResources/StandardMacros.IncrementInt` (`self.SpawnedPlayers`))
    (:`  `
      (return (`self.Selected Player Start`)))))

(fn `FindPlayerStart`
  (params (Player :type "Controller Object Reference") (IncomingName :type String))
  (returns (ReturnValue :type "Actor Object Reference"))
  (locals (PlayerNumber :type String))
  (return Player))

(fn `GetDefaultPawnClassForController`
  (params (InController :type "Controller Object Reference"))
  (returns (ReturnValue :type "Object Class Reference"))
  (bind _returnvalue (`parent.GetDefaultPawnClassForController` null))
  (return _returnvalue))

(fn `GetPlayerStartPoints`
  (bind _outactors (`GameplayStatics.GetAllActorsOfClass` "/Script/Engine.PlayerStart"))
  (set `self.PlayerStartArray` _outactors))

(fn `NewFunction_0`)

(fn `ReadyToStartMatch`
  (returns (ReturnValue :type Boolean))
  (return false))

(fn `SetPlayerInitialRotations`
  ;[1 1 1] -Get each player;
  ; -Change controller to respond to normal vector values;
  ; // This is because the player start has been rotated for each
  ; player and the controls will not be aligned otherwise;
  (`KismetSystemLibrary.PrintString` "Setting Player Initial Rotation" true true (struct :`G` 0.66 :`B` 1.0 :`A` 1.0) 10.0)
  (`Controller.SetControlRotation` (`GameplayStatics.GetPlayerController` 0) (`KismetMathLibrary.Conv_Vector4ToRotator` (`KismetMathLibrary.MakeVector4` 0.0))))

(fn `SpawnDefaultPawnAtTransform`
  (params (NewPlayer :type "Controller Object Reference") (SpawnTransform :type "Transform Structure (by ref)"))
  (returns (ReturnValue :type "Pawn Object Reference"))
  (return null))

(fn `SpawnDefaultPawnFor`
  (params (NewPlayer :type "Controller Object Reference") (StartSpot :type "Actor Object Reference"))
  (returns (ReturnValue :type "Pawn Object Reference"))
  (return null))

(fn `SpawnPlayers`
  (bind _index (`self.Index`))
  ;[0.4158 1 0.9701] Array is zero based, update for normal 1-4 use.
  (for _index_2 (range (`self.MaxPlayerCount`))
    (set `self.Index` _index_2)
    ;[0.4374 1 0.9901] Assign each player from the array with the player start tag
    (for _array_element (`self.PlayerStartArray`)
      (if (== (`PlayerStart.PlayerStartTag` _array_element) (`KismetStringLibrary.Conv_StringToName` (`KismetStringLibrary.Conv_IntToString` (`self.Index`))))
        ;[0.4256 1 0.9602] Spawn the BP_Player and assign the player to posses it
        (`GameplayStatics.CreatePlayer` (`self.Index`))
        (bind _returnvalue (`|SpawnActorFromClass` "/Game/Blueprints/BP_Player_Character.BP_Player_Character_C" (`self.GetTransform` _array_element) "Undefined" "OverrideRootScale" null null))
        (`Controller.Possess` (`GameplayStatics.GetPlayerController` _index) _returnvalue)
        ;[1 1 1] Add each unique element to the players array
        (`KismetArrayLibrary.Array_AddUnique` (`self.Players`) _returnvalue)
        ;[0.2696 0.9602 1] Change the mesh and animations based on player index
        (switch `int` _index
          (:`0`
            (`SkinnedMeshComponent.SetSkinnedAssetAndUpdate` (`Character.Mesh` _returnvalue) "/Game/OLD_Assets/Animations/Bear/Bear_IdleAnim.Bear_IdleAnim" true)
            ;[1 1 1] Player Colour Indicators
            (`PrimitiveComponent.SetMaterial` (`/Game/Blueprints/BP_Player_Character.Cone` _returnvalue) 0 "/Game/OLD_Assets/Player_Colours/Cyan_Mat.Cyan_Mat")
            (`PrimitiveComponent.SetMaterial` (`/Game/Blueprints/BP_Player_Character.ConeTop` _returnvalue) 0 "/Game/OLD_Assets/Player_Colours/Cyan_Mat.Cyan_Mat"))
          (:`1`
            (bind _mesh (`Character.Mesh` _returnvalue))
            (`SkinnedMeshComponent.SetSkinnedAssetAndUpdate` _mesh "/Game/OLD_Assets/Animations/Fox/Fox_IdleAnim.Fox_IdleAnim" true)
            (`SkeletalMeshComponent.K2_SetAnimInstanceClass` _mesh "/Game/OLD_Assets/Animations/Fox/Fox_ANIM_BP.Fox_ANIM_BP_C")
            (`PrimitiveComponent.SetMaterial` (`/Game/Blueprints/BP_Player_Character.Cone` _returnvalue) 0 "/Game/OLD_Assets/Player_Colours/red_Mat.red_Mat")
            (`PrimitiveComponent.SetMaterial` (`/Game/Blueprints/BP_Player_Character.ConeTop` _returnvalue) 0 "/Game/OLD_Assets/Player_Colours/red_Mat.red_Mat"))
          (:`2`
            (bind _mesh_2 (`Character.Mesh` _returnvalue))
            (`SkinnedMeshComponent.SetSkinnedAssetAndUpdate` _mesh_2 "/Game/OLD_Assets/Animations/Penguin/Penguin_IdleAnim.Penguin_IdleAnim" true)
            (`SkeletalMeshComponent.K2_SetAnimInstanceClass` _mesh_2 "/Game/OLD_Assets/Animations/Penguin/PenguinBP.PenguinBP_C")
            (`PrimitiveComponent.SetMaterial` (`/Game/Blueprints/BP_Player_Character.Cone` _returnvalue) 0 "/Game/OLD_Assets/Player_Colours/yellow_Mat.yellow_Mat")
            (`PrimitiveComponent.SetMaterial` (`/Game/Blueprints/BP_Player_Character.ConeTop` _returnvalue) 0 "/Game/OLD_Assets/Player_Colours/yellow_Mat.yellow_Mat"))
          (:`3`
            (bind _mesh_3 (`Character.Mesh` _returnvalue))
            (`SkinnedMeshComponent.SetSkinnedAssetAndUpdate` _mesh_3 "/Game/OLD_Assets/Animations/Walrus/Walrus_NEW_IdleAnim.Walrus_NEW_IdleAnim" true)
            (`SkeletalMeshComponent.K2_SetAnimInstanceClass` _mesh_3 "/Game/OLD_Assets/Animations/Walrus/Walrus_ANIM_BP.Walrus_ANIM_BP_C")
            (`PrimitiveComponent.SetMaterial` (`/Game/Blueprints/BP_Player_Character.Cone` _returnvalue) 0 "/Game/OLD_Assets/Player_Colours/purple_Mat.purple_Mat")
            (`PrimitiveComponent.SetMaterial` (`/Game/Blueprints/BP_Player_Character.ConeTop` _returnvalue) 0 "/Game/OLD_Assets/Player_Colours/purple_Mat.purple_Mat")))))))

(fn `UserConstructionScript`)