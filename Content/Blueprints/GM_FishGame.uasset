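; Game mode for the fish minigame, handling local multiplayer setup, a countdown timer and the winner reveal.
; InitialiseGame spawns a character per player at its index-tagged PlayerStart, applies that player's husky look and resets control rotations.
; InitTimer starts a looping timer that counts down to OnTimesUp, which flags game over and blends player one's view to the personal camera.
; That camera targets the top scorer, found by indexing GetAllActorsOfClass with the highest GameInstance score's index.
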(event `OnTimesUp`
  (`KismetSystemLibrary.PrintString` "Time's up")
  (bind _asbp_game_instance (cast `/Game/Blueprints/BP_GameInstance` (`GameplayStatics.GetGameInstance`)))
  (bind (_indexofmaxvalue _maxvalue) (`KismetMathLibrary.MaxOfIntArray` (`|MakeArray` (`/Game/Blueprints/BP_GameInstance.Player1Score` _asbp_game_instance) (`/Game/Blueprints/BP_GameInstance.Player2Score` _asbp_game_instance) (`/Game/Blueprints/BP_GameInstance.Player3Score` _asbp_game_instance) (`/Game/Blueprints/BP_GameInstance.Player4Score` _asbp_game_instance))))
  (set `self.WinningPlayer` _indexofmaxvalue)
  (set `self.GameOver?` true)
  ;[1 1 1] Get the winning player number
  (bind _outactors (`GameplayStatics.GetAllActorsOfClass` "/Game/Blueprints/BP_Player_Character.BP_Player_Character_C"))
  ;[1 1 1] Get the personal camera actor and update it
  (bind _outactors_2 (`GameplayStatics.GetAllActorsOfClass` "/Game/Blueprints/Cameras/BP_PersonalCamera.BP_PersonalCamera_C"))
  (bind _output (`|GetArrayItem` _outactors_2))
  (`/Game/Blueprints/Cameras/BP_PersonalCamera.UpdatePersonalCamera` _output (`|GetArrayItem` _outactors (`KismetStringLibrary.Conv_StringToInt` (`KismetTextLibrary.Conv_TextToString` (`KismetTextLibrary.Conv_IntToText` _indexofmaxvalue)))))
  ;[1 1 1] Transition the camera to the winner
  (`PlayerController.SetViewTargetWithBlend` (`GameplayStatics.GetPlayerController` 0) _output 1.0 "VTBlend_EaseIn" 1.0 false))

(event `OnTimerTick`)

(event `InitialiseGame`
  (`|ExecutionSequence`
    (:`then_0`
      (`self.GetPlayerStartPoints`))
    (:`then_1`
      (`self.SpawnPlayers`))
    (:`then_2`
      (`self.SetPlayerInitialRotations`))))

(fn `GetPlayerStartPoints`
  (bind _outactors (`GameplayStatics.GetAllActorsOfClass` "/Script/Engine.PlayerStart"))
  (set `self.PlayerStartArray` _outactors))

(fn `Init Timer`
  (params (`Time To Complete` :type "Float (double-precision)" :default 0.0))
  (set `self.Time Remaining` `Time To Complete`)
  (bind _returnvalue (`KismetSystemLibrary.K2_SetTimer` null "Refresh Timer" (`self.Timer Tick Delta`) true))
  (set `self.Main Timer Handle` _returnvalue))

(fn `Refresh Timer`
  (bind _output_get (set `self.Time Remaining` (- (`self.Time Remaining`) (`self.Timer Tick Delta`))))
  (if (<= _output_get 0.0)
    (`self.OnTimesUp`)
    (else
      (`self.OnTimerTick`))))

(fn `SetPlayerInitialRotations`
  ;[1 1 1] -Get each player;
  ; -Change controller to respond to normal vector values;
  ; // This is because the player start has been rotated for each
  ; player and the controls will not be aligned otherwise;
  (bind _outactors (`GameplayStatics.GetAllActorsOfClass` "/Game/Blueprints/BP_Player_Character.BP_Player_Character_C"))
  (for (_ _array_index) _outactors
    (`Controller.SetControlRotation` (`GameplayStatics.GetPlayerController` _array_index) (`KismetMathLibrary.Conv_Vector4ToRotator` (`KismetMathLibrary.MakeVector4` 0.0)))))

(fn `SpawnPlayers`
  (bind _index (`self.Index`))
  (bind _asbp_game_instance (cast `/Game/Blueprints/BP_GameInstance` (`GameplayStatics.GetGameInstance`)))
  ;[0.4158 1 0.9701] Array is zero based, update for normal 1-4 use.
  (for _index_2 (range (`/Game/Blueprints/BP_GameInstance.TotalPlayers` _asbp_game_instance))
    (set `self.Index` _index_2)
    ;[0.4374 1 0.9901] Assign each player from the array with the player start tag
    (for _array_element (`self.PlayerStartArray`)
      (if (== (`PlayerStart.PlayerStartTag` _array_element) (`KismetStringLibrary.Conv_StringToName` (`KismetStringLibrary.Conv_IntToString` (`self.Index`))))
        ;[0.4256 1 0.9602] Spawn the BP_Player and assign the player to posses it
        (bind _returnvalue (`GameplayStatics.CreatePlayer` (`self.Index`)))
        (bind _returnvalue_2 (`|SpawnActorFromClass` "/Game/Blueprints/BP_Player_Character.BP_Player_Character_C" (`self.GetTransform` _array_element) "Undefined" "OverrideRootScale" _returnvalue null))
        (`Controller.Possess` (`GameplayStatics.GetPlayerController` _index) _returnvalue_2)
        ;[1 1 1] Add each unique element to the players array
        (`KismetArrayLibrary.Array_AddUnique` (`self.Players`) _returnvalue_2)
        ;[0.2696 0.9602 1] Change the mesh and animations based on player index
        (switch `int` _index
          (:`0`
            (bind _mesh (`Character.Mesh` _returnvalue_2))
            (`SkinnedMeshComponent.SetSkinnedAssetAndUpdate` _mesh "/Game/NEW_Assets/Characters/FairyHusky/Animations/FairyHuskyIdle_anim.FairyHuskyIdle_anim" true)
            (`SkeletalMeshComponent.K2_SetAnimInstanceClass` _mesh "/Game/NEW_Assets/Characters/FairyHusky/Animations/ABP_Fairy.ABP_Fairy_C")
            (`StaticMeshComponent.SetStaticMesh` (`/Game/Blueprints/BP_Player_Character.PlayerIndicator ` _returnvalue_2) "/Game/Assets/Crystals/Crystal_FairyHusky.Crystal_FairyHusky")
            (set `/Game/Blueprints/BP_Player_Character.PlayerNumber` 0 _returnvalue_2)
            (`ParticleSystemComponent.SetTemplate` (`/Game/Blueprints/BP_Player_Character.DashParticles` _returnvalue_2) "/Game/Assets/Materials/DashReady/DashReady_Fairy_Particle.DashReady_Fairy_Particle"))
          (:`1`
            (bind _mesh_2 (`Character.Mesh` _returnvalue_2))
            (`SkinnedMeshComponent.SetSkinnedAssetAndUpdate` _mesh_2 "/Game/NEW_Assets/Characters/HuskMitri/Animations/HuskmitriIdle_anim.HuskmitriIdle_anim" true)
            (`SkeletalMeshComponent.K2_SetAnimInstanceClass` _mesh_2 "/Game/NEW_Assets/Characters/HuskMitri/Animations/ABP_HuskMitri.ABP_HuskMitri_C")
            (`StaticMeshComponent.SetStaticMesh` (`/Game/Blueprints/BP_Player_Character.PlayerIndicator ` _returnvalue_2) "/Game/Assets/Crystals/Crystal_HuskyMitri.Crystal_HuskyMitri")
            (set `/Game/Blueprints/BP_Player_Character.PlayerNumber` 1 _returnvalue_2)
            (`ParticleSystemComponent.SetTemplate` (`/Game/Blueprints/BP_Player_Character.DashParticles` _returnvalue_2) "/Game/Assets/Materials/DashReady/DashReady_Huskmitri_Particle.DashReady_Huskmitri_Particle"))
          (:`2`
            (bind _mesh_3 (`Character.Mesh` _returnvalue_2))
            (`SkinnedMeshComponent.SetSkinnedAssetAndUpdate` _mesh_3 "/Game/NEW_Assets/Characters/PunkHusky/PunkHuskyIdle_anim.PunkHuskyIdle_anim" true)
            (`SkeletalMeshComponent.K2_SetAnimInstanceClass` _mesh_3 "/Game/NEW_Assets/Characters/PunkHusky/ABP_Punk.ABP_Punk_C")
            (`StaticMeshComponent.SetStaticMesh` (`/Game/Blueprints/BP_Player_Character.PlayerIndicator ` _returnvalue_2) "/Game/Assets/Crystals/Crystal_HuskyPunk.Crystal_HuskyPunk")
            (set `/Game/Blueprints/BP_Player_Character.PlayerNumber` 2 _returnvalue_2)
            (`ParticleSystemComponent.SetTemplate` (`/Game/Blueprints/BP_Player_Character.DashParticles` _returnvalue_2) "/Game/Assets/Materials/DashReady/DashReady_Punk_Particle.DashReady_Punk_Particle"))
          (:`3`
            (bind _mesh_4 (`Character.Mesh` _returnvalue_2))
            (`SkinnedMeshComponent.SetSkinnedAssetAndUpdate` _mesh_4 "/Game/NEW_Assets/Characters/SwimmerHusky/SwimmerHuskyIdle_anim.SwimmerHuskyIdle_anim" true)
            (`SkeletalMeshComponent.K2_SetAnimInstanceClass` _mesh_4 "/Game/NEW_Assets/Characters/SwimmerHusky/ABP_Swimmer.ABP_Swimmer_C")
            (`StaticMeshComponent.SetStaticMesh` (`/Game/Blueprints/BP_Player_Character.PlayerIndicator ` _returnvalue_2) "/Game/Assets/Crystals/Crystal_HuskySwimmer.Crystal_HuskySwimmer")
            (set `/Game/Blueprints/BP_Player_Character.PlayerNumber` 3 _returnvalue_2)
            (`ParticleSystemComponent.SetTemplate` (`/Game/Blueprints/BP_Player_Character.DashParticles` _returnvalue_2) "/Game/Assets/Materials/DashReady/DashReady_Swimmer_Particle.DashReady_Swimmer_Particle")))))))

(fn `UserConstructionScript`)