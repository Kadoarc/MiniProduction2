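; BP_PersonalCamera is a camera actor that tracks one of two characters, FISH or HOTPOTATO, from above and facing opposite to it.
; UpdatePersonalCamera uses LevelOne to choose the character and latch its update flag.
; Tick reuses that event's move node, snapping to the character's location with a height offset and reversed yaw.
; Neither flag is cleared here, so FISH takes priority once set.
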(event `UpdatePersonalCamera`
  (params (Char_FISH :type "/Game/Blueprints/BP_Player_Character Object Reference") (Char_HOTPOTATO :type "/Game/Blueprints/BP_Player_Character_HotPotato Object Reference") (`LevelOne?` :type Boolean))
  (bind (_returnvalue_x _returnvalue_y _returnvalue_z) (`KismetMathLibrary.BreakVector` (`self.K2_GetActorLocation` Char_HOTPOTATO)))
  (bind (_returnvalue_roll _returnvalue_pitch _returnvalue_yaw) (`KismetMathLibrary.BreakRotator` (`self.K2_GetActorRotation` Char_HOTPOTATO)))
  (bind (_returnvalue_x_2 _returnvalue_y_2 _returnvalue_z_2) (`KismetMathLibrary.BreakVector` (`self.K2_GetActorLocation` Char_FISH)))
  (bind (_returnvalue_roll_2 _returnvalue_pitch_2 _returnvalue_yaw_2) (`KismetMathLibrary.BreakRotator` (`self.K2_GetActorRotation` Char_FISH)))
  (if `LevelOne?`
    (set `self.ShouldUpdate_1?` true)
    (`self.K2_SetActorLocationAndRotation` (`KismetMathLibrary.MakeVector` _returnvalue_x_2 _returnvalue_y_2 (+ _returnvalue_z_2 80.0)) (`KismetMathLibrary.MakeRotator` _returnvalue_roll_2 _returnvalue_pitch_2 (- _returnvalue_yaw_2 180.0)) :!label _label)
    (else
      (set `self.ShouldUpdate_2?` true)
      (`self.K2_SetActorLocationAndRotation` (`KismetMathLibrary.MakeVector` _returnvalue_x _returnvalue_y (+ _returnvalue_z 80.0)) (`KismetMathLibrary.MakeRotator` _returnvalue_roll _returnvalue_pitch (- _returnvalue_yaw 180.0)) :!label _label_2))))

(event `self.ReceiveTick`
  (params (DeltaSeconds :type "Float (single-precision)"))
  (if (`self.ShouldUpdate_1?`)
    (goto _label)
    (elif (`self.ShouldUpdate_2?`)
      (goto _label_2))))

(fn `UserConstructionScript`)