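; Local multiplayer game mode that spawns the players, runs a start countdown and announces the winning score when time runs out.
; BeginPlay creates a player per GameInstance TotalPlayers at index-tagged PlayerStarts, assigns each a mesh, AnimBP and colour, then resets control rotations.
; A looping Delay counts down with only player 0's input disabled.
; InitTimer, not called here, starts the match timer, which waits for the countdown and prints the highest score on expiry.
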(event `OnTimesUp`
  (`KismetSystemLibrary.PrintString` "Time's up")
  (bind _asbp_game_instance (cast `/Game/Blueprints/BP_GameInstance` (`GameplayStatics.GetGameInstance`)))
  (`KismetSystemLibrary.PrintText` (`KismetTextLibrary.Conv_StringToText` (`KismetStringLibrary.Concat_StrStr` "Winning Score:" (`KismetTextLibrary.Conv_TextToString` (`KismetTextLibrary.Conv_IntToText` (`.MaxValue` (`KismetMathLibrary.MaxOfIntArray` (`|MakeArray` (`/Game/Blueprints/BP_GameInstance.Player1Score` _asbp_game_instance) (`/Game/Blueprints/BP_GameInstance.Player2Score` _asbp_game_instance) (`/Game/Blueprints/BP_GameInstance.Player3Score` _asbp_game_instance) (`/Game/Blueprints/BP_GameInstance.Player4Score` _asbp_game_instance))))))))))

(event `OnTimerTick`)

(event `self.ReceiveBeginPlay`
  (bind _returnvalue (`GameplayStatics.GetPlayerController` 0))
  (bind _intcountdown (`self.IntCountdown`))
  (`|ExecutionSequence`
    (:`then_0`
      (`self.GetPlayerStartPoints`)
      (`self.SpawnPlayers`))
    (:`then_1`
      (`self.SetPlayerInitialRotations`))
    (:`then_2`
      (bind _asbp_player_character (cast `/Game/Blueprints/BP_Player_Character` (`GameplayStatics.GetPlayerCharacter` 0))
        (:`then`
          (`self.DisableInput` _asbp_player_character _returnvalue)
          (`KismetSystemLibrary.Delay` 1.0 :!label _label)
          (`KismetSystemLibrary.PrintString` (`KismetStringLibrary.Conv_IntToString` _intcountdown))
          (if (== _intcountdown 0)
            (`self.EnableInput` _asbp_player_character _returnvalue)
            (else
              (set `self.IntCountdown` (- _intcountdown 1))
              (goto _label))))
        (:`CastFailed`
          (`KismetSystemLibrary.PrintString` "Failed"))))))

(event `CustomEvent`)

(fn `GetPlayerStartPoints`
  (bind _outactors (`GameplayStatics.GetAllActorsOfClass` "/Script/Engine.PlayerStart"))
  (set `self.PlayerStartArray` _outactors))

(fn `Init Timer`
  (params (`Time To Complete` :type "Float (double-precision)" :default 0.0))
  (set `self.Time Remaining` `Time To Complete`)
  (bind _returnvalue (`KismetSystemLibrary.K2_SetTimer` null "Refresh Timer" (`self.Timer Tick Delta`) true))
  (set `self.Main Timer Handle` _returnvalue))

(fn `Refresh Timer`
  (if (== (`self.IntCountdown`) 0)
    (bind _output_get (set `self.Time Remaining` (- (`self.Time Remaining`) (`self.Timer Tick Delta`))))
    (if (<= _output_get 0.0)
      (`self.OnTimesUp`)
      (else
        (`self.OnTimerTick`)))
    (else
      (set `self.Time Remaining` (`self.Time Remaining`)))))

(fn `SetPlayerInitialRotations`
  ;[1 1 1] -Get each player;
  ; -Change controller to respond to normal vector values;
  ; // This is because the player start has been rotated for each
  ; player and the controls will not be aligned otherwise;
  (bind _outactors (`GameplayStatics.GetAllActorsOfClass` "/Game/Blueprints/BP_Player_Character.BP_Player_Character_C"))
  (for (_ _array_index) _outactors
    (`Controller.SetControlRotation` (`GameplayStatics.GetPlayerController` _array_index) (`KismetMathLibrary.Conv_Vector4ToRotator` (`KismetMathLibrary.MakeVector4` 0.0)))))

(fn `SpawnPlayers`
  (bind _index (`self.Index`))
  (bind _asbp_game_instance (cast `/Game/Blueprints/BP_GameInstance` (`GameplayStatics.GetGameInstance`)))
  ;[0.4158 1 0.9701] Array is zero based, update for normal 1-4 use.
  (for _index_2 (range (`/Game/Blueprints/BP_GameInstance.TotalPlayers` _asbp_game_instance))
    (set `self.Index` _index_2)
    ;[0.4374 1 0.9901] Assign each player from the array with the player start tag
    (for _array_element (`self.PlayerStartArray`)
      (if (== (`PlayerStart.PlayerStartTag` _array_element) (`KismetStringLibrary.Conv_StringToName` (`KismetStringLibrary.Conv_IntToString` (`self.Index`))))
        ;[0.4256 1 0.9602] Spawn the BP_Player and assign the player to posses it
        (bind _returnvalue (`GameplayStatics.CreatePlayer` -1))
        (bind _returnvalue_2 (`|SpawnActorFromClass` "/Game/Blueprints/BP_Player_Character.BP_Player_Character_C" (`self.GetTransform` _array_element) "Undefined" "OverrideRootScale" _returnvalue null))
        (`Controller.Possess` (`GameplayStatics.GetPlayerController` _index) _returnvalue_2)
        ;[1 1 1] Add each unique element to the players array
        (`KismetArrayLibrary.Array_AddUnique` (`self.Players`) _returnvalue_2)
        ;[0.2696 0.9602 1] Change the mesh and animations based on player index
        (switch `int` _index
          (:`0`
            (bind _mesh (`Character.Mesh` _returnvalue_2))
            (`SkinnedMeshComponent.SetSkinnedAssetAndUpdate` _mesh "/Game/NEW_Assets/Characters/FairyHusky/Animations/FairyHuskyIdle_anim.FairyHuskyIdle_anim" true)
            (`SkeletalMeshComponent.K2_SetAnimInstanceClass` _mesh "/Game/NEW_Assets/Characters/FairyHusky/Animations/ABP_Fairy.ABP_Fairy_C")
            ;[1 1 1] Player Colour Indicators
            (`PrimitiveComponent.SetMaterial` (`/Game/Blueprints/BP_Player_Character.Cone` _returnvalue_2) 0 "/Game/OLD_Assets/Player_Colours/Cyan_Mat.Cyan_Mat")
            (`PrimitiveComponent.SetMaterial` (`/Game/Blueprints/BP_Player_Character.ConeTop` _returnvalue_2) 0 "/Game/OLD_Assets/Player_Colours/Cyan_Mat.Cyan_Mat"))
          (:`1`
            (bind _mesh_2 (`Character.Mesh` _returnvalue_2))
            (`SkinnedMeshComponent.SetSkinnedAssetAndUpdate` _mesh_2 "/Game/NEW_Assets/Characters/HuskMitri/Animations/HuskmitriIdle_anim.HuskmitriIdle_anim" true)
            (`SkeletalMeshComponent.K2_SetAnimInstanceClass` _mesh_2 "/Game/NEW_Assets/Characters/HuskMitri/Animations/ABP_HuskMitri.ABP_HuskMitri_C")
            (`PrimitiveComponent.SetMaterial` (`/Game/Blueprints/BP_Player_Character.Cone` _returnvalue_2) 0 "/Game/OLD_Assets/Player_Colours/red_Mat.red_Mat")
            (`PrimitiveComponent.SetMaterial` (`/Game/Blueprints/BP_Player_Character.ConeTop` _returnvalue_2) 0 "/Game/OLD_Assets/Player_Colours/red_Mat.red_Mat"))
          (:`2`
            (bind _mesh_3 (`Character.Mesh` _returnvalue_2))
            (`SkinnedMeshComponent.SetSkinnedAssetAndUpdate` _mesh_3 "/Game/NEW_Assets/Characters/PunkHusky/PunkHuskyIdle_anim.PunkHuskyIdle_anim" true)
            (`SkeletalMeshComponent.K2_SetAnimInstanceClass` _mesh_3 "/Game/NEW_Assets/Characters/PunkHusky/ABP_Punk.ABP_Punk_C")
            (`PrimitiveComponent.SetMaterial` (`/Game/Blueprints/BP_Player_Character.Cone` _returnvalue_2) 0 "/Game/OLD_Assets/Player_Colours/yellow_Mat.yellow_Mat")
            (`PrimitiveComponent.SetMaterial` (`/Game/Blueprints/BP_Player_Character.ConeTop` _returnvalue_2) 0 "/Game/OLD_Assets/Player_Colours/yellow_Mat.yellow_Mat"))
          (:`3`
            (bind _mesh_4 (`Character.Mesh` _returnvalue_2))
            (`SkinnedMeshComponent.SetSkinnedAssetAndUpdate` _mesh_4 "/Game/NEW_Assets/Characters/SwimmerHusky/SwimmerHuskyIdle_anim.SwimmerHuskyIdle_anim" true)
            (`SkeletalMeshComponent.K2_SetAnimInstanceClass` _mesh_4 "/Game/NEW_Assets/Characters/SwimmerHusky/ABP_Swimmer.ABP_Swimmer_C")
            (`PrimitiveComponent.SetMaterial` (`/Game/Blueprints/BP_Player_Character.Cone` _returnvalue_2) 0 "/Game/OLD_Assets/Player_Colours/purple_Mat.purple_Mat")
            (`PrimitiveComponent.SetMaterial` (`/Game/Blueprints/BP_Player_Character.ConeTop` _returnvalue_2) 0 "/Game/OLD_Assets/Player_Colours/purple_Mat.purple_Mat")))))))

(fn `UserConstructionScript`)