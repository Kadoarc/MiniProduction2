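; Collectible fish for a four-player iceberg game that players grab to score points.
; On BeginPlay it launches its skeletal mesh with a random-strength impulse toward a random TargetPoint in the level.
; Box overlap by a player increments that player's GameInstance score, destroys the fish and spawns a FishyBoi at a random low position on either side of the iceberg.
; A separate actor-level overlap also destroys it on player contact, without scoring.
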(event `self.ReceiveActorBeginOverlap`
  (params (OtherActor :type "Actor Object Reference"))
  (bind _asbp_player_character (cast `/Game/Blueprints/BP_Player_Character` OtherActor))
  (`self.K2_DestroyActor`))

(event `self.ReceiveBeginPlay`
  (bind _outactors (`GameplayStatics.GetAllActorsOfClass` "/Script/Engine.TargetPoint"))
  (bind _output_get (set `self.TargetPointArray` _outactors))
  (`PrimitiveComponent.AddImpulse` (`self.SkeletalMesh`) (* (`KismetMathLibrary.GetDirectionUnitVector` (`self.K2_GetActorLocation`) (`self.K2_GetActorLocation` (`|GetArrayItem` _output_get (`KismetMathLibrary.RandomIntegerInRange` 0 (- (`KismetArrayLibrary.Array_Length` _output_get) 1))))) (`KismetMathLibrary.RandomFloatInRange` 300000.0 450000.0)) "None" false))

(event `SpawnFishyBoi`
  (if (`KismetMathLibrary.RandomBool`)
    ;[0.006914 0.9203 1] Spawn on the Left of the iceberg
    (`|SpawnActorFromClass` "/Game/Blueprints/FishyBoi.FishyBoi_C" (`KismetMathLibrary.MakeTransform` (`KismetMathLibrary.MakeVector` (`KismetMathLibrary.RandomFloatInRange` -1600.0 1600.0) (`KismetMathLibrary.RandomFloatInRange` -1600.0 -2200.0) -900.0)) "Undefined" "OverrideRootScale" null null)
    (else
      ;[0.006914 0.9203 1] Spawn on the Right of the iceberg
      (`|SpawnActorFromClass` "/Game/Blueprints/FishyBoi.FishyBoi_C" (`KismetMathLibrary.MakeTransform` (`KismetMathLibrary.MakeVector` (`KismetMathLibrary.RandomFloatInRange` -1200.0 1400.0) (`KismetMathLibrary.RandomFloatInRange` 1900.0 2600.0) -900.0)) "Undefined" "OverrideRootScale" null null))))

(event `self.Box.OnComponentBeginOverlap`
  (params (OverlappedComponent :type "PrimitiveComponent Object Reference") (OtherActor :type "Actor Object Reference") (OtherComp :type "PrimitiveComponent Object Reference") (OtherBodyIndex :type Integer) (bFromSweep :type Boolean) (SweepResult :type "HitResult Structure (by ref)"))
  ;[1 1 1] When the fish is collected
  (`|ExecutionSequence`
    (:`then_0`
      (bind _asbp_player_character (cast `/Game/Blueprints/BP_Player_Character` OtherActor))
      (switch `int` (`/Game/Blueprints/BP_Player_Character.PlayerNumber` _asbp_player_character)
        (:`0`
          (bind _asbp_game_instance (cast `/Game/Blueprints/GameModes/BP_GameInstance` (`GameplayStatics.GetGameInstance`)))
          (bind _result (`/Engine/EditorBlueprintResources/StandardMacros.IncrementInt` (stale _output_get))
            (:`  `
              (bind _output_get (set `/Game/Blueprints/GameModes/BP_GameInstance.Player1Score` _result _asbp_game_instance))
              (`self.K2_DestroyActor`))))
        (:`1`
          (bind _asbp_game_instance_2 (cast `/Game/Blueprints/GameModes/BP_GameInstance` (`GameplayStatics.GetGameInstance`)))
          (bind _result_2 (`/Engine/EditorBlueprintResources/StandardMacros.IncrementInt` (stale _output_get_2))
            (:`  `
              (bind _output_get_2 (set `/Game/Blueprints/GameModes/BP_GameInstance.Player2Score` _result_2 _asbp_game_instance_2))
              (`self.K2_DestroyActor`))))
        (:`2`
          (bind _asbp_game_instance_3 (cast `/Game/Blueprints/GameModes/BP_GameInstance` (`GameplayStatics.GetGameInstance`)))
          (bind _result_3 (`/Engine/EditorBlueprintResources/StandardMacros.IncrementInt` (stale _output_get_3))
            (:`  `
              (bind _output_get_3 (set `/Game/Blueprints/GameModes/BP_GameInstance.Player3Score` _result_3 _asbp_game_instance_3))
              (`self.K2_DestroyActor`))))
        (:`3`
          (bind _asbp_game_instance_4 (cast `/Game/Blueprints/GameModes/BP_GameInstance` (`GameplayStatics.GetGameInstance`)))
          (bind _result_4 (`/Engine/EditorBlueprintResources/StandardMacros.IncrementInt` (stale _output_get_4))
            (:`  `
              (bind _output_get_4 (set `/Game/Blueprints/GameModes/BP_GameInstance.Player4Score` _result_4 _asbp_game_instance_4))
              (`self.K2_DestroyActor`)))))
      (`self.SpawnFishyBoi`))))

(fn `UserConstructionScript`)