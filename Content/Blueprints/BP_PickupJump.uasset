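; Collectible pickup that awards a point to the player who touches it and can move along a spline as a jumping fish.
; When ActiveFish is set, BeginPlay runs a timeline, scaled by Duration and started at FishStartOffset, that drives location and rotation along the referenced spline.
; On overlap with a player character, it increments that player's score in BP_GameInstance by PlayerNumber, supporting four players, then destroys itself.
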(event `self.ReceiveBeginPlay`
  (if (`self.ActiveFish`)
    (`self.JumpingFishObj`)))

(event `JumpingFishObj`
  (bind _returnvalue (`KismetMathLibrary.Lerp` 0.0 (`SplineComponent.GetSplineLength` (`/Game/Blueprints/Track.UsefulSpline` (`self.SplineRef`))) (`self.Alpha`)))
  (`TimelineComponent.SetPlayRate` (`self.JumpingFish`) (/ 1.0 (`self.Duration`)))
  (`TimelineComponent.SetNewTime` (`self.JumpingFish`) (`self.FishStartOffset`))
  (bind (_direction _alpha) (`Timeline|JumpingFish`)
    (:`Update`
      (set `self.Alpha` _alpha)
      (`self.K2_SetActorLocationAndRotation` (`SplineComponent.GetLocationAtDistanceAlongSpline` (`/Game/Blueprints/Track.UsefulSpline` (`self.SplineRef`)) _returnvalue "World") (`SplineComponent.GetRotationAtDistanceAlongSpline` (`/Game/Blueprints/Track.UsefulSpline` (`self.SplineRef`)) _returnvalue "World")))))

(event `self.Collision.OnComponentBeginOverlap`
  (params (OverlappedComponent :type "PrimitiveComponent Object Reference") (OtherActor :type "Actor Object Reference") (OtherComp :type "PrimitiveComponent Object Reference") (OtherBodyIndex :type Integer) (bFromSweep :type Boolean) (SweepResult :type "HitResult Structure (by ref)"))
  (bind _asbp_player_character (cast `/Game/Blueprints/BP_Player_Character` OtherActor))
  (switch `int` (`/Game/Blueprints/BP_Player_Character.PlayerNumber` _asbp_player_character)
    (:`0`
      (bind _asbp_game_instance (cast `/Game/Blueprints/BP_GameInstance` (`GameplayStatics.GetGameInstance`)))
      (bind _result (`/Engine/EditorBlueprintResources/StandardMacros.IncrementInt` (stale _output_get))
        (:`  `
          (bind _output_get (set `/Game/Blueprints/BP_GameInstance.Player1Score` _result _asbp_game_instance))
          (`self.K2_DestroyActor`))))
    (:`1`
      (bind _asbp_game_instance_2 (cast `/Game/Blueprints/BP_GameInstance` (`GameplayStatics.GetGameInstance`)))
      (bind _result_2 (`/Engine/EditorBlueprintResources/StandardMacros.IncrementInt` (stale _output_get_2))
        (:`  `
          (bind _output_get_2 (set `/Game/Blueprints/BP_GameInstance.Player2Score` _result_2 _asbp_game_instance_2))
          (`self.K2_DestroyActor`))))
    (:`2`
      (bind _asbp_game_instance_3 (cast `/Game/Blueprints/BP_GameInstance` (`GameplayStatics.GetGameInstance`)))
      (bind _result_3 (`/Engine/EditorBlueprintResources/StandardMacros.IncrementInt` (stale _output_get_3))
        (:`  `
          (bind _output_get_3 (set `/Game/Blueprints/BP_GameInstance.Player3Score` _result_3 _asbp_game_instance_3))
          (`self.K2_DestroyActor`))))
    (:`3`
      (bind _asbp_game_instance_4 (cast `/Game/Blueprints/BP_GameInstance` (`GameplayStatics.GetGameInstance`)))
      (bind _result_4 (`/Engine/EditorBlueprintResources/StandardMacros.IncrementInt` (stale _output_get_4))
        (:`  `
          (bind _output_get_4 (set `/Game/Blueprints/BP_GameInstance.Player4Score` _result_4 _asbp_game_instance_4))
          (`self.K2_DestroyActor`))))))

(fn `UserConstructionScript`)